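; Punch Gameplay Ability that plays the attack montage and applies GE_Damage to whatever the punch hits.
; While the montage plays, it waits once for a Weapon.Hit gameplay event, expected via the AN_Punch anim notify, and uses the payload's target data.
; The ability ends when the montage completes, blends out or is interrupted.
; On end, it terminates the stored wait task if still valid.
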(event Ability|EventActivateAbility
  ;[1 1 1] Play a punch animation, see if it hits anything, apply damage effect if it does
  (Animation|Montage|PlayMontage (.skeletalmeshcomponent (Ability|GetActorInfo)) "/Game/Mannequin/Animations/M_Attack.M_Attack" ; This can trigger an AN_Punch event in the ThirdPersonCharcter
    (:then
      (bind (_asynctaskproxy _payload) (Ability|Tasks|WaitGameplayEvent "(TagName=\"Weapon.Hit\")" 0 true) ; This comes back here if the AN works
        (:then
          (Variables|Default|SetAsyncTask_WaitForHit _asynctaskproxy))
        (:EventReceived
          (GameplayEffects|ApplyGameplayEffectToTarget (.TargetData (Utilities|Struct|BreakGameplayEventData _payload)) "/Game/Abilities/GE_Damage.GE_Damage_C" 1 1)
          (Development|PrintString "Punch hit: Triggering GE_Damage"))))
    (:OnCompleted
      (Ability|EndAbility :!label _label) ; If the montages finishes, and we don't hit anything, the event can't fire, so we end the ability
    )
    (:OnBlendOut
      (goto _label))
    (:OnInterrupted
      (goto _label))))

(event Ability|EventOnEndAbility
  (params (bWasCancelled :type Boolean))
  (bind _asynctask_waitforhit (Variables|Default|GetAsyncTask_WaitForHit))
  (Utilities|IsValid _asynctask_waitforhit
    (:Is%20Valid
      (GameplayTasks|EndTask _asynctask_waitforhit))))